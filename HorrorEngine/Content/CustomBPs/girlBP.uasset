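; GirlBP is an AI-driven figure that follows the player, turning its static mesh to face them every tick.
; When starting at the world origin, it retries random navmesh points around the player until one exceeds a minimum distance and a spawned probe actor's root reports not visible.
; It teleports there at player height, waits a set lifetime, then spawns a replacement at the origin and destroys itself, repeating the cycle.
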(event Collision|EventActorBeginOverlap
  (params (OtherActor :type Actor%20Object%20Reference)))

(event EventTick
  (params (DeltaSeconds :type Float%20%28single-precision%29))
  (bind _staticmesh (Variables|Default|GetStaticMesh))
  (Transformation|SetWorldRotation _staticmesh (Math|Rotator|MakeRotator 0.0 0.0 (- (.yaw (Math|Rotator|FindLookatRotation (Transformation|GetWorldLocation _staticmesh) (Transformation|GetActorLocation (Game|GetPlayerCharacter 0)))) 9e+01)) false false)
  (AI|AIMoveTo self "0, 0, 0" (Game|GetPlayerCharacter 0) 5.0 false))

(event EventBeginPlay
  (bind _returnvalue (Game|GetPlayerCharacter 0))
  (bind _returnvalue_2 (Transformation|GetActorLocation _returnvalue))
  (Pawn|SpawnDefaultController)
  (if (Math|Vector|Equal(Vector) (Transformation|GetActorLocation self) "0, 0, 0" 0.0001)
    (bind (_randomlocation _returnvalue_3) (Class|NavigationSystemV1|GetRandomLocationinNavigableRadius _returnvalue_2 (Variables|Default|GetMaxSpawnDistance) 0 0 :!label _label))
    ;[1 1 1] doesPointExist
    (if _returnvalue_3
      (if (> (Math|Vector|Distance(Vector) _randomlocation _returnvalue_2) (Variables|Default|GetMinSpawnDistance))
        (bind _returnvalue_4 (Game|SpawnActorfromClass "/Script/Engine.Actor" (Math|Conversions|ToTransform(Vector) (Math|Vector|MakeVector (.X (Math|Vector|BreakVector _randomlocation)) (.Y (Math|Vector|BreakVector _randomlocation)) (.Z (Math|Vector|BreakVector _returnvalue_2)))) "AlwaysSpawn" 0 0))
        (if (Rendering|IsVisible (Variables|/Script/Engine.Actor|GetRootComponent _returnvalue_4))
          (goto _label)
          (else
            (Transformation|SetActorLocation (Math|Vector|MakeVector (.X (Math|Vector|BreakVector _randomlocation)) (.Y (Math|Vector|BreakVector _randomlocation)) (.Z (Math|Vector|BreakVector _returnvalue_2))) false false)
            (Utilities|FlowControl|Delay (Variables|Default|GetTimeBeforeAutoDestroy))
            (Game|SpawnActorfromClass "girlBP_C" (Math|Transform|MakeTransform "0, 0, 0") "AlwaysSpawn" 0 0)
            (Actor|DestroyActor)))
        (else
          (goto _label))))))

(fn ConstructionScript)