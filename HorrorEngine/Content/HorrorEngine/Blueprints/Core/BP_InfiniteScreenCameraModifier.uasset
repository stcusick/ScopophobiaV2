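; BP_InfiniteScreenCameraModifier is a camera modifier that applies Tobii Infinite Screen (extended view) rotation to the player camera.
; It caches the unmodified view location and rotation, then combines that rotation with the Tobii angles, leaving location and FOV unchanged.
; An optional smooth step on camera pitch scales the yaw offset.
; When Infinite Screen is disabled, it zeroes the stored angles and passes the view through.
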(fn BlueprintModifyCamera
  (params (DeltaTime :type Float%20%28single-precision%29) (ViewLocation :type Vector :default "0, 0, 0") (ViewRotation :type Rotator :default "0, 0, 0") (FOV :type Float%20%28single-precision%29))
  (bind _returnvalue (Class|TobiiBlueprintLibrary|GetTobiiInfiniteScreenAngles))
  (bind (_roll _pitch _yaw) (Math|Rotator|BreakRotator _returnvalue))
  (Variables|InfiniteScreenProperties|SetViewLocationWithoutExtendedView ViewLocation)
  (bind _output_get (Variables|InfiniteScreenProperties|SetViewRotationWithoutExtendedView ViewRotation))
  (if (Class|TobiiInteractionsBlueprintLibrary|IsInfiniteScreenEnabled)
    (if (Variables|InfiniteScreenProperties|GetScaleExtendedViewByInputPitch)
      (bind _returnvalue_2 (Class|TobiiInteractionsBlueprintLibrary|CalculateSmoothPitchStep (.Pitch (Math|Rotator|BreakRotator _output_get))))
      (Variables|InfiniteScreenProperties|SetInfiniteScreenAngles (Math|Rotator|MakeRotator _roll _pitch (* _returnvalue_2 _yaw)))
      (else
        (Variables|InfiniteScreenProperties|SetInfiniteScreenAngles _returnvalue)))
    (bind _returnvalue_3 (Class|TobiiInteractionsBlueprintLibrary|MakeInfiniteScreenCameraRotator (Variables|InfiniteScreenProperties|GetViewRotationWithoutExtendedView) (Variables|InfiniteScreenProperties|GetInfiniteScreenAngles)))
    (return ViewLocation _returnvalue_3 FOV)
    (else
      (Variables|InfiniteScreenProperties|SetInfiniteScreenAngles "0, 0, 0")
      (return ViewLocation ViewRotation FOV))))